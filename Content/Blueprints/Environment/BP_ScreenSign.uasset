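; BP_ScreenSign is a placeable environment screen sign with a mesh and a rect light.
; Its construction script picks one of two sign meshes from an enum.
; An On flag either applies the chosen light intensity and color or sets the intensity to zero.
; The event graph holds only disabled placeholder events, so the setup has no runtime logic.
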(event EventBeginPlay)

(event Collision|EventActorBeginOverlap
  (params (OtherActor :type Actor%20Object%20Reference)))

(event EventTick
  (params (DeltaSeconds :type Float%20%28single-precision%29)))

(fn ConstructionScript
  (bind _rectlight (Variables|Default|GetRectLight))
  (Components|StaticMesh|SetStaticMesh (Variables|Default|GetStaticMesh) (Utilities|Select :Index (Variables|Default|GetEnum_Sign) :NewEnumerator0 "/Game/Mesh/EnvArtModules/ScreenSignA.ScreenSignA" :NewEnumerator1 "/Game/Mesh/EnvArtModules/ScreenSignB.ScreenSignB"))
  (if (Variables|Default|GetbOn)
    (Rendering|Components|Light|SetIntensity _rectlight (Variables|Default|GetIntensity))
    (Rendering|Components|Light|SetLightColor _rectlight (Variables|Default|GetLightColor) true)
    (else
      (Rendering|Components|Light|SetIntensity _rectlight 0.0))))